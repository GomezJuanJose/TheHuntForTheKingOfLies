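; Dialogue event that plays a time segment of a Level Sequence cinematic when triggered.
; It searches for a level sequence actor tagged as a dialogue cinematic, reusing it if the asset matches and destroying it otherwise.
; Without a match, it creates a new tagged sequence player.
; The player pauses, moves to the start second and plays to the end second using configurable update methods, so successive events can share one cinematic.
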(event `self.RecieveEventTriggered`
  (params (ConsideringPlayer :type "PlayerController Object Reference") (NPCActor :type "Actor Object Reference"))
  ;[1 1 1] Try to find the same sequencer, if its the case then reuse it and play the segment if its not the same the destroy it, create a new one and play the segment, if theres none found then create a new one and play the segment
  (set `self.HasFoundSameSequence` false)
  (bind _outactors (`GameplayStatics.GetAllActorsOfClass` "/Script/LevelSequence.LevelSequenceActor"))
  (for _array_element _outactors
    (if (`Actor.ActorHasTag` _array_element "Sequence.DialogCinematic")
      (if (== (`LevelSequenceActor.LevelSequenceAsset` _array_element) (`self.Cinematic`))
        (`self.PlaySequenceSegment` (`LevelSequenceActor.SequencePlayer` _array_element))
        (set `self.HasFoundSameSequence` true)
        (break)
        (else
          (`Actor.K2_DestroyActor` _array_element)
          (set `self.HasFoundSameSequence` false)
          (break)))))
  (if (not (`self.HasFoundSameSequence`))
    (bind (_outactor _returnvalue) (`LevelSequencePlayer.CreateLevelSequencePlayer` (`self.Cinematic`)))
    (set `Actor.Tags` (`|MakeArray` "Sequence.DialogCinematic" :!type "Name") _outactor)
    (`self.PlaySequenceSegment` _returnvalue)))

(fn `PlaySequenceSegment`
  (params (SceneSequence :type "MovieSceneSequencePlayer Object Reference"))
  (`MovieSceneSequencePlayer.Pause` SceneSequence)
  (`MovieSceneSequencePlayer.SetPlaybackPosition` SceneSequence (make `MovieSceneSequencePlaybackParams` (struct :`FrameNumber` (struct)) (`self.StartSecond`) "" "Time" (`self.StartBlendMethod`)))
  (`MovieSceneSequencePlayer.PlayTo` :`self` SceneSequence :`PlaybackParams` (make `MovieSceneSequencePlaybackParams` (struct :`FrameNumber` (struct)) (`self.EndSecond`) "" "Time" (`self.EndBlendMethod`))))