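; Dialogue event Blueprint that plays an animation montage on a character when triggered during a dialogue.
; A flag picks the target: the NPC actor, or the interactor obtained through the NPC's dialogue component interface.
; The target is cast to Character, and its mesh AnimInstance plays the montage with configurable blend-in and play rate, then jumps to the configured start section.
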(event `self.RecieveEventTriggered`
  (params (ConsideringPlayer :type "PlayerController Object Reference") (NPCActor :type "Actor Object Reference"))
  (bind _anim_montage (`self.Anim Montage`))
  (bind _anim_montage_2 (`self.Anim Montage`))
  (if (`self.IsForInteractor?`)
    (bind _returnvalue (message `IDialogueComponent.GetInteractor` (`|GetArrayItem` (`Actor.GetComponentsByInterface` NPCActor "/Script/ALSV4_CPP.IDialogueComponent"))))
    (bind _ascharacter (cast `Character` _returnvalue))
    (bind _returnvalue_2 (`SkeletalMeshComponent.GetAnimInstance` (`Character.Mesh` _ascharacter)))
    (`AnimInstance.Montage_PlayWithBlendIn` _returnvalue_2 _anim_montage (make `AlphaBlendArgs` null (`self.Blend Time`) (`self.Blend Option`)) (`self.Play Rate`) "MontageLength" 0.0 true)
    (`AnimInstance.Montage_JumpToSection` _returnvalue_2 (`self.Start Section Name`) _anim_montage)
    (else
      (bind _ascharacter_2 (cast `Character` NPCActor))
      (bind _returnvalue_3 (`SkeletalMeshComponent.GetAnimInstance` (`Character.Mesh` _ascharacter_2)))
      (`AnimInstance.Montage_PlayWithBlendIn` _returnvalue_3 _anim_montage_2 (make `AlphaBlendArgs` null (`self.Blend Time`) (`self.Blend Option`)) (`self.Play Rate`) "MontageLength" 0.0 true)
      (`AnimInstance.Montage_JumpToSection` _returnvalue_3 (`self.Start Section Name`) _anim_montage_2))))