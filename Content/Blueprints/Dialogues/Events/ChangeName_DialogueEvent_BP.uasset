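; Dialogue event that renames the NPC it is triggered on to its Name variable.
; It rebuilds the full name through the NPC's IDialogueComponent with no nickname, then updates the HUD's Talk interaction prompt.
; It also rewrites the component's interactable data with the new name, keeping the other fields, so the prompt stays correct when the NPC is next in interaction range.
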(event `self.RecieveEventTriggered`
  (params (ConsideringPlayer :type "PlayerController Object Reference") (NPCActor :type "Actor Object Reference"))
  (bind _name (`self.Name`))
  (bind _returnvalue (`KismetTextLibrary.Conv_NameToText` _name))
  (bind _output (`|GetArrayItem` (`Actor.GetComponentsByInterface` NPCActor "/Script/ALSV4_CPP.IDialogueComponent")))
  (message `IDialogueComponent.ConstructFullName` _output _name "None")
  ;[0 0.3073 0] Updates the name of the interactable dialog component for the notification show on the HUD & its data struct when its in his interact range again
  (bind _widget (message `/Game/Blueprints/Interfaces/IHUD_Basic.GetWidget` (`PlayerController.GetHUD` (`GameplayStatics.GetPlayerController` 0))))
  (message `/Game/Blueprints/Interfaces/UI/IHUDAnimations_BP.UpdateInteractActionNotify` _widget _returnvalue "Talk")
  (bind _interactablestruct (message `IInteractable_Basic.GetInteractableData_Basic` _output))
  (message `IInteractable_Basic.SetInteractableData_Basic` _output (make `InteractableData_Basic` _returnvalue (`.InteractionCategory` (break `InteractableData_Basic` _interactablestruct)) (`.bDisableOnInteract` (break `InteractableData_Basic` _interactablestruct)) (`.TimeToRenable` (break `InteractableData_Basic` _interactablestruct)) (`.bAttachedSound` (break `InteractableData_Basic` _interactablestruct)) (`.InteractSoundCue` (break `InteractableData_Basic` _interactablestruct)))))