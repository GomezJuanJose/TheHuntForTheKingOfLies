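; Dialogue event that stops an animation montage on a Character when triggered during a dialogue.
; IsForInteractor selects the target: the interactor, fetched through the NPC's IDialogueComponent interface component, or the NPC actor itself.
; The target is cast to Character, and its mesh anim instance stops AnimMontage using the configured blend-out time and blend option.
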(event `self.RecieveEventTriggered`
  (params (ConsideringPlayer :type "PlayerController Object Reference") (NPCActor :type "Actor Object Reference"))
  (if (`self.IsForInteractor?`)
    (bind _returnvalue (message `IDialogueComponent.GetInteractor` (`|GetArrayItem` (`Actor.GetComponentsByInterface` NPCActor "/Script/ALSV4_CPP.IDialogueComponent"))))
    (bind _ascharacter (cast `Character` _returnvalue))
    (`AnimInstance.Montage_StopWithBlendOut` (`SkeletalMeshComponent.GetAnimInstance` (`Character.Mesh` _ascharacter)) (make `AlphaBlendArgs` null (`self.Blend Time`) (`self.Blend Option`)) (`self.Anim Montage`))
    (else
      (bind _ascharacter_2 (cast `Character` NPCActor))
      (`AnimInstance.Montage_StopWithBlendOut` (`SkeletalMeshComponent.GetAnimInstance` (`Character.Mesh` _ascharacter_2)) (make `AlphaBlendArgs` null (`self.Blend Time`) (`self.Blend Option`)) (`self.Anim Montage`)))))