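; Blueprint function library for interface text that turns an input key into a short label for button prompts.
; GetShortKeyName compares the key through a chain of branches covering Space and common gamepad buttons, triggers and stick clicks.
; Most matches return rich-text styled names pairing PlayStation and Xbox labels, while special buttons and stick clicks return plain text.
; Any other key falls back to its engine display name.
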(fn `Get Short Key Name`
  (params (Key :type "Key Structure" :default "SpaceBar"))
  (returns (Name :type Text))
  (if (== Key "SpaceBar")
    (return "<Default_i>SPACE</>")
    (elif (== Key "Gamepad_RightShoulder")
      (return "<Default_i>R1</> or <Default_i>RT</>")
      (elif (== Key "Gamepad_RightTriggerAxis")
        (return "<Default_i>R2</> or <Default_i>RB</>")
        (elif (== Key "Gamepad_LeftShoulder")
          (return "<Default_i>L1</> or <Default_i>LT</>")
          (elif (== Key "Gamepad_LeftTriggerAxis")
            (return "<Default_i>L2</> or <Default_i>LB</>")
            (elif (== Key "Gamepad_FaceButton_Bottom")
              (return "<Default_i>X</> or <Default_i>A</>")
              (elif (== Key "Gamepad_FaceButton_Right")
                (return "<Default_i>O</> or <Default_i>B</>")
                (elif (== Key "Gamepad_FaceButton_Left")
                  (return "<Default_i>SQUARE</> or <Default_i>X</>")
                  (elif (== Key "Gamepad_FaceButton_Top")
                    (return "<Default_i>TRIANGLE</> or <Default_i>Y</>")
                    (elif (== Key "Gamepad_Special_Right")
                      (return "SPECIAL RIGHT")
                      (elif (== Key "Gamepad_Special_Left")
                        (return "SPECIAL LEFT")
                        (elif (== Key "Gamepad_RightThumbstick")
                          (return "R3")
                          (elif (== Key "Gamepad_LeftThumbstick")
                            (return "L3")
                            (else
                              (return (`KismetInputLibrary.Key_GetDisplayName` Key)))))))))))))))))