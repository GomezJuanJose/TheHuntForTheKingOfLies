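; Interface manager component that puts the main menu and pause menu widgets on the player's screen.
; On BeginPlay it creates the main menu intro widget and clears the HUD's pause-message flag.
; SetPause creates the pause menu and sets that flag, only if no top-level instance exists, preventing duplicates from rapid clicks.
; An unconnected time-dilation node remains from a planned slow-motion pause.
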(event `self.ReceiveBeginPlay`
  (`self.SetMainMenu`))

(event `self.SetPause`
  (params (Pause :type Boolean))
  (bind _pausemenubackgroundclass (`self.PauseMenuBackgroundClass`))
  ;[0.01591 0.3802 0] Its not performance intense due uses a Hash table and always will be only 1 instance of the class so the temporal cost is O(1)
  ;;[0 0.07812 0.002474] Avoids to create more than one pause menu when clicks quickly the resume and pause button
  (bind _foundwidgets (`WidgetBlueprintLibrary.GetAllWidgetsOfClass` _pausemenubackgroundclass))
  (if (`KismetArrayLibrary.Array_IsEmpty` _foundwidgets)
    (bind _returnvalue (`|CreateWidget` _pausemenubackgroundclass))
    (`UserWidget.AddToPlayerScreen` _returnvalue 0)
    (message `/Game/Blueprints/Interfaces/IHUD_Basic.SetIsPause` (`PlayerController.GetHUD` (`GameplayStatics.GetPlayerController` 0)) true)))

(event `self.SetMainMenu`
  (bind _returnvalue (`|CreateWidget` (`self.MainMenuBackgroundIntroClass`)))
  (`UserWidget.AddToPlayerScreen` _returnvalue 0)
  (message `/Game/Blueprints/Interfaces/IHUD_Basic.SetIsPause` (`PlayerController.GetHUD` (`GameplayStatics.GetPlayerController` 0)) false))