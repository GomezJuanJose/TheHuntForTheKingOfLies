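; Interact component that shows or hides the HUD's interaction prompt for the actor passed to its UpdateHUDBP event.
; It reads name and category through IInteractable_Basic from the actor, or failing that from its first implementing component, defaulting to "???" with no category.
; The data goes to the widget obtained from player 0's HUD, and an invalid actor hides the prompt.
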(event `self.UpdateHUDBP`
  (params (Actor :type "Actor Object Reference"))
  (bind _returnvalue (`Actor.GetComponentsByInterface` Actor "/Script/ALSV4_CPP.IInteractable_Basic"))
  (bind _returnvalue_2 (`GameplayStatics.GetPlayerController` 0))
  (bind (_auxinteractable_struct_name _auxinteractable_struct_interactioncategory) (break `InteractableData_Basic` (`self.AuxInteractable Struct`)))
  (bind _returnvalue_3 (`PlayerController.GetHUD` _returnvalue_2))
  (`parent.UpdateHUDBP` Actor)
  (`/Engine/EditorBlueprintResources/StandardMacros.IsValid` Actor
    (:`Is Valid`
      ;[0 0.2448 0.002448] Checks if the actor implements the interactable interface, if not checks if any component has the interface, in that case gets the first one
      (if (`KismetSystemLibrary.DoesImplementInterface` Actor "/Script/ALSV4_CPP.IInteractable_Basic")
        (bind _interactablestruct (message `IInteractable_Basic.GetInteractableData_Basic` Actor))
        (set `self.AuxInteractable Struct` _interactablestruct)
        (elif (`KismetArrayLibrary.Array_IsNotEmpty` _returnvalue)
          (bind _interactablestruct_2 (message `IInteractable_Basic.GetInteractableData_Basic` (`|GetArrayItem` _returnvalue)))
          (set `self.AuxInteractable Struct` _interactablestruct_2)
          (else
            (set `self.AuxInteractable Struct` (make `InteractableData_Basic` "???" "None")))))
      (bind _widget (message `/Game/Blueprints/Interfaces/IHUD_Basic.GetWidget` (`PlayerController.GetHUD` (`GameplayStatics.GetPlayerController` 0))))
      (message `/Game/Blueprints/Interfaces/UI/IHUDAnimations_BP.ShowInteractActionNotify` _widget true)
      (message `/Game/Blueprints/Interfaces/UI/IHUDAnimations_BP.UpdateInteractActionNotify` _widget _auxinteractable_struct_name _auxinteractable_struct_interactioncategory))
    (:`Is Not Valid`
      (`/Engine/EditorBlueprintResources/StandardMacros.IsValid` _returnvalue_2
        (:`Is Valid`
          (`/Engine/EditorBlueprintResources/StandardMacros.IsValid` _returnvalue_3
            (:`Is Valid`
              (bind _widget_2 (message `/Game/Blueprints/Interfaces/IHUD_Basic.GetWidget` _returnvalue_3))
              (message `/Game/Blueprints/Interfaces/UI/IHUDAnimations_BP.ShowInteractActionNotify` _widget_2 false))))))))