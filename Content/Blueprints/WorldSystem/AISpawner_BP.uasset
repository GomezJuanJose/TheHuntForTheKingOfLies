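; AI spawner Blueprint that shows or hides a fire effect to reflect whether the spawner is enabled.
; On each world time event it calls the parent logic, then checks the enabled flag in its basic spawner data.
; A Dissapear timeline runs in reverse or forward to drive the fire's scale and Light parameter.
; Two DoOnce gates, reset according to the flag when the timeline finishes, prevent repeated transitions.
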(event `self.ExecuteTimeEvent`
  (params (Hour :type Integer) (Wheater :type "EWeatherType Enum" :default "ClearSky"))
  (bind _aispawnerdata_basic_benabledspawner (break `AISpawnerData_Basic` (`self.AISpawnerData_Basic`)))
  (bind _p_fire (`self.P_Fire`))
  (`parent.ExecuteTimeEvent` Hour Wheater)
  ;[0 0.2865 0] Enables or disables the fire when the spawner is active or not
  (if _aispawnerdata_basic_benabledspawner
    (`/Engine/EditorBlueprintResources/StandardMacros.DoOnce` false :!label _label
      (:`Completed`
        (bind (_direction _scale) (`Timeline|Dissapear` :!via `Reverse` :!label _label_2)
          (:`Update`
            (`SceneComponent.SetWorldScale3D` _p_fire _scale)
            (`FXSystemComponent.SetFloatParameter` _p_fire "Light" (* (.x _scale) 10.0)))
          (:`Finished`
            (if _aispawnerdata_basic_benabledspawner
              (goto _label_3 :!via `Reset`)
              (else
                (goto _label :!via `Reset`)))))))
    (else
      (`/Engine/EditorBlueprintResources/StandardMacros.DoOnce` false :!label _label_3
        (:`Completed`
          (goto _label_2))))))

(fn `UserConstructionScript`)