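; Interactable craft station world object that opens a crafting interface for the player.
; On the interface event it runs the parent logic, creates the widget, adds it to the player screen, then passes it the station and its crafting list.
; The construction script slaves modular body-part meshes (foot, legs, head, body, hands, shoulders) to one skeletal component via master pose, so they share its pose.
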(event `self.CreateCraftstationInterface`
  (`parent.CreateCraftstationInterface`)
  (bind _returnvalue (`|CreateWidget` (`self.CraftstateInterface`)))
  (`UserWidget.AddToPlayerScreen` _returnvalue 0)
  (message `/Game/Blueprints/Interfaces/UI/ICraftstationMenu_BP.SetCraftstationContext` _returnvalue self)
  (message `/Game/Blueprints/Interfaces/UI/ICraftstationMenu_BP.SetGraftList` _returnvalue (`self.CraftingList`)))

(fn `UserConstructionScript`
  (`SkinnedMeshComponent.SetLeaderPoseComponent` (`self.Foot`) (`self.PlaceActorSkeletalComponent`) false)
  (`SkinnedMeshComponent.SetLeaderPoseComponent` (`self.Legs`) (`self.PlaceActorSkeletalComponent`) false)
  (`SkinnedMeshComponent.SetLeaderPoseComponent` (`self.Head`) (`self.PlaceActorSkeletalComponent`) false)
  (`SkinnedMeshComponent.SetLeaderPoseComponent` (`self.Body`) (`self.PlaceActorSkeletalComponent`) false)
  (`SkinnedMeshComponent.SetLeaderPoseComponent` (`self.Hands`) (`self.PlaceActorSkeletalComponent`) false)
  (`SkinnedMeshComponent.SetLeaderPoseComponent` (`self.Shoulders`) (`self.PlaceActorSkeletalComponent`) false))