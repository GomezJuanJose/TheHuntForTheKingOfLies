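; General HUD Blueprint that creates the player's HUD widget on BeginPlay and acts as the access point for controlling it.
; A timeline plays or reverses to fade the crosshair, pushing opacity to the widget.
; PlayFade runs the widget's fade, waits for its returned time, then shows the HUD on forward or hides it on reverse.
; It also exposes direct show/hide, a widget getter, and a stored pause flag.
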(event `self.ReceiveBeginPlay`
  (`self.CreateWidget`))

(event `PlayCrossFade`
  (bind (_direction _crosshairopacity) (`Timeline|CrosshairOpacity` :!label _label)
    (:`Update`
      (`self.UpdateCrossOpacity` _crosshairopacity))))

(event `ReverseCrossFade`
  (goto _label :!via `Reverse`))

(event `/Game/Blueprints/Interfaces/IHUD_Basic.SetIsPause`
  (params (IsPause :type Boolean))
  (set `self.IsPause` IsPause))

(event `/Game/Blueprints/Interfaces/IHUD_Basic.PlayFade`
  (params (PlayMode :type "EUMGSequencePlayMode Enum" :default "Forward"))
  (bind _hudwidgetbp (`self.HUDWidgetBP`))
  (bind _animationtime (`/Game/Blueprints/Widgets/HUD_Widget.PlayFade` (`self.HUDWidgetBP`) PlayMode))
  (switch `EUMGSequencePlayMode` PlayMode
    (:`Forward`
      (`KismetSystemLibrary.Delay` _animationtime)
      (`/Game/Blueprints/Widgets/HUD_Widget.ShowHUD` _hudwidgetbp true))
    (:`Reverse`
      (`KismetSystemLibrary.Delay` _animationtime)
      (`/Game/Blueprints/Widgets/HUD_Widget.ShowHUD` _hudwidgetbp false))))

(event `/Game/Blueprints/Interfaces/IHUD_Basic.ShowHUDWidget`
  (params (Show :type Boolean))
  (`/Game/Blueprints/Widgets/HUD_Widget.ShowHUD` (`self.HUDWidgetBP`) Show))

(fn `CreateWidget`
  (bind _returnvalue (`|CreateWidget` (`self.HUDClass`) (`GameplayStatics.GetPlayerController` 0)))
  (`UserWidget.AddToPlayerScreen` _returnvalue 0)
  (set `self.HUDWidgetBP` _returnvalue))

(fn `GetIsPause`
  (returns (IsPause :type Boolean))
  (return (`self.IsPause`)))

(fn `GetWidget`
  (returns (Widget :type "UserWidget Object Reference"))
  (return (`self.HUDWidgetBP`)))

(fn `UpdateCrossOpacity`
  (params (Opacity :type "Float (double-precision)"))
  (`/Game/Blueprints/Widgets/HUD_Widget.UpdateCrossOpacity` (`self.HUDWidgetBP`) Opacity))

(fn `UserConstructionScript`)